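; BP_Blocks is an actor that builds and manages a grid of damageable blocks.
; Its construction script adds a BP_BlockComponent for each cell, spaced by Padding and tagged with its grid position.
; A Hit on one of these components applies one point of damage through HitBlock, which fires the OnBlockDestroyed dispatcher with the block's position when it is destroyed.
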(event `self.ReceiveHit`
  (params (MyComp :type "PrimitiveComponent Object Reference") (Other :type "Actor Object Reference") (OtherComp :type "PrimitiveComponent Object Reference") (bSelfMoved :type Boolean) (HitLocation :type "Vector Structure") (HitNormal :type "Vector Structure") (NormalImpulse :type "Vector Structure") (Hit :type "HitResult Structure (by ref)"))
  (bind _asbp_block_component (cast `/Game/Actors/BP_BlockComponent` MyComp))
  (`self.HitBlock` _asbp_block_component))

(fn `HitBlock`
  (params (`Block Component` :type "/Game/Actors/BP_BlockComponent Object Reference"))
  (locals (WasDestroy :type Boolean :default false) (BlockPosition :type "Vector2D Structure"))
  (set `local.BlockPosition` (`/Game/Actors/BP_BlockComponent.Position` `Block Component`))
  (`/Game/Actors/BP_BlockComponent.ApplyDamage` `Block Component` 1 (`local.WasDestroy`))
  (if (`local.WasDestroy`)
    (`KismetSystemLibrary.PrintString` "Block destroyed" true true (struct :`R` 1.0 :`B` 0.97442 :`A` 1.0))
    (`self.OnBlockDestroyed` (`local.BlockPosition`))
    (else
      (`KismetSystemLibrary.PrintString` "Block NOT destroyed" true true (struct :`R` 1.0 :`B` 0.97442 :`A` 1.0)))))

(fn `UserConstructionScript`
  (for _index (range (+ (`self.X`) 1))
    (for _index_2 (range (+ (`self.Y`) 1))
      (`AddComponent|NODE_AddBP_BlockComponent-0` :`RelativeTransform` (`KismetMathLibrary.MakeTransform` (`KismetMathLibrary.MakeVector` (`KismetMathLibrary.Conv_IntToDouble` (* _index (`self.Padding`))) (`KismetMathLibrary.Conv_IntToDouble` (* _index_2 (`self.Padding`))))) :`Position` (`KismetMathLibrary.MakeVector2D` (`KismetMathLibrary.Conv_IntToDouble` _index) (`KismetMathLibrary.Conv_IntToDouble` _index_2))))))