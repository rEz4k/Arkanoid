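; BP_BlockComponent is a destructible block component that takes damage and can drop a bonus pickup.
; ApplyDamage subtracts from Life, reports whether the block was destroyed, and swaps to a pebbled cobblestone material while it survives.
; At zero Life or below, DropBonus randomly spawns a BP_Bonus at the block's transform before the component destroys itself.
; The component also binds to OnDestroyCalled at BeginPlay to destroy itself when that event fires.
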(event `self.ReceiveBeginPlay`
  (`parent.ReceiveBeginPlay`)
  (add `self.OnDestroyCalled` (delegate `OnDestroyCalled_Event`)))

(event `OnDestroyCalled_Event`
  (`self.K2_DestroyComponent`))

(fn `ApplyDamage`
  (params (Damage :type Integer) (bWasDestroyed :type "Boolean (by ref)"))
  (bind _output_get (set `self.Life` (- (`self.Life`) Damage)))
  (bind _returnvalue (<= _output_get 0))
  (`|VariableSetRef` bWasDestroyed _returnvalue)
  (if _returnvalue
    (`self.DropBonus`)
    (`self.K2_DestroyComponent`)
    (else
      (`self.SetMaterial` 0 "/Game/StarterContent/Materials/M_CobbleStone_Pebble.M_CobbleStone_Pebble"))))

(fn `DropBonus`
  (if (> (`KismetMathLibrary.RandomIntegerInRange` 1 10) 7)
    (`|SpawnActorFromClass` "/Game/Actors/BP_Bonus.BP_Bonus_C" (`self.K2_GetComponentToWorld`) "AlwaysSpawn" "OverrideRootScale" null null)))