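; BP_Ball is a ball actor that moves at a set speed along a direction and bounces off whatever blocks it.
; Each tick it makes a swept world offset in X and Y only, reflecting Direction about the hit normal on a blocking hit.
; Overlapping a KillZVolume sets WillDead and calls the OnDead dispatcher, and Tick destroys the actor once that flag is set.
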(event `self.ReceiveActorBeginOverlap`
  (params (OtherActor :type "Actor Object Reference"))
  (cast `KillZVolume` OtherActor)
  (set `self.bWillDead` true)
  (`self.OnDead`))

(event `self.ReceiveTick`
  (params (DeltaSeconds :type "Float (single-precision)"))
  (bind (_returnvalue_x _returnvalue_y) (`KismetMathLibrary.BreakVector` (* (* (`self.Direction`) (`self.Speed`)) DeltaSeconds)))
  (`|ExecutionSequence`
    (:`then_0`
      (bind _sweephitresult (`self.K2_AddActorWorldOffset` (`KismetMathLibrary.MakeVector` _returnvalue_x _returnvalue_y) true))
      (bind (_bblockinghit _binitialoverlap _time _distance _location _impactpoint _normal) (`GameplayStatics.BreakHitResult` _sweephitresult))
      (if _bblockinghit
        (set `self.Direction` (`KismetMathLibrary.GetReflectionVector` (`self.Direction`) _normal))))
    (:`then_1`
      (if (`self.bWillDead`)
        (`self.K2_DestroyActor`)))))

(fn `IsWillDead`
  (returns (WillDead :type Boolean))
  (return (`self.bWillDead`)))

(fn `UserConstructionScript`)