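; BP_First is an actor with a Cube component that destroys another actor after a set number of collisions.
; Each blocking hit on the Cube increments Clash, and when it equals CountClash the actor from that hit is destroyed.
; The counter is shared across all hit actors and never resets, so the destruction triggers only on that exact count.
; BeginPlay, overlap, Tick and construction only call their parent implementations.
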(event `self.ReceiveBeginPlay`
  (`parent.ReceiveBeginPlay`))

(event `self.ReceiveActorBeginOverlap`
  (params (OtherActor :type "Actor Object Reference"))
  (`parent.ReceiveActorBeginOverlap` OtherActor))

(event `self.ReceiveTick`
  (params (DeltaSeconds :type "Float (single-precision)"))
  (`parent.ReceiveTick` DeltaSeconds))

(event `self.Cube.OnComponentHit`
  (params (HitComponent :type "PrimitiveComponent Object Reference") (OtherActor :type "Actor Object Reference") (OtherComp :type "PrimitiveComponent Object Reference") (NormalImpulse :type "Vector Structure") (Hit :type "HitResult Structure (by ref)"))
  (bind (_bblockinghit _binitialoverlap _time _distance _location _impactpoint _normal _impactnormal _physmat _hitactor) (`GameplayStatics.BreakHitResult` Hit))
  (if _bblockinghit
    (set `self.Clash` (+ (`self.Clash`) 1))
    (if (== (`self.Clash`) (`self.CountClash`))
      (`self.K2_DestroyActor` _hitactor))))

(fn `UserConstructionScript`
  (`parent.UserConstructionScript`))