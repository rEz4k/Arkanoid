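; BP_Second is an actor that shrinks each time its Cube component registers a blocking hit.
; The Cube's hit event subtracts a fixed step from the whole actor's 3D scale, with no lower limit.
; BeginPlay, overlap and the construction script only call their parents, and Tick is disabled.
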(event `self.ReceiveBeginPlay`
  (`parent.ReceiveBeginPlay`))

(event `self.ReceiveActorBeginOverlap`
  (params (OtherActor :type "Actor Object Reference"))
  (`parent.ReceiveActorBeginOverlap` OtherActor))

(event `self.Cube.OnComponentHit`
  (params (HitComponent :type "PrimitiveComponent Object Reference") (OtherActor :type "Actor Object Reference") (OtherComp :type "PrimitiveComponent Object Reference") (NormalImpulse :type "Vector Structure") (Hit :type "HitResult Structure (by ref)"))
  (if (`GameplayStatics.BreakHitResult` Hit)
    (`self.SetActorScale3D` (- (`self.GetActorScale3D`) 0.05))))

(fn `UserConstructionScript`
  (`parent.UserConstructionScript`))