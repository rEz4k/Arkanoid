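; Player pawn for a ball game with lives: it moves sideways in fixed swept steps from axis input and spawns BP_Ball at its capsule on BeginPlay.
; Each spawned ball's OnDead event is bound, and OnBallDead counts balls not flagged as dying.
; When none remain, it subtracts a life, then either spawns a new ball or prints Game Over, reporting status through debug prints.
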(event `self.ReceiveBeginPlay`
  (`self.SpawnBall`))

(event `InputAxis|Sideways movement`
  (params (AxisValue :type "Float (single-precision)"))
  (if (< AxisValue 0.0)
    (`self.K2_AddActorWorldOffset` (35.0 0.0 0.0) true)))

(event `InputAxis|Sideways movement`
  (params (AxisValue :type "Float (single-precision)"))
  (if (> AxisValue 0.0)
    (`self.K2_AddActorWorldOffset` (-35.0 0.0 0.0) true)))

(fn `OnBallDead`
  (locals (LivesBalls :type Integer))
  (bind _outactors (`GameplayStatics.GetAllActorsOfClass` "/Game/Actors/BP_Ball.BP_Ball_C"))
  (for _array_element _outactors
    (if (not (`/Game/Actors/BP_Ball.IsWillDead` _array_element))
      (bind _result (`/Engine/EditorBlueprintResources/StandardMacros.IncrementInt` (`local.LivesBalls`))
        (:`  `
          (`KismetSystemLibrary.PrintString` (`KismetStringLibrary.Concat_StrStr` "Number of live balls: " (`KismetStringLibrary.Conv_IntToString` _result)) true true (struct :`G` 0.66 :`B` 1.0 :`A` 1.0) 3.0)))))
  (if (== (`local.LivesBalls`) 0)
    (`KismetSystemLibrary.PrintString` "All balls dead" true true (struct :`R` 0.5625 :`G` 0.150387 :`B` 0.111328 :`A` 1.0) 3.0)
    (`self.SubstructLife`)
    (if (== (`self.Life`) 0)
      (`KismetSystemLibrary.PrintString` (`KismetStringLibrary.Concat_StrStr` "Game Over, Maaan! \nGame Over, Maaan! \nGame Over, Maaan!") true true (struct :`R` 0.410178 :`G` 0.142295 :`B` 0.546875 :`A` 1.0) 5.0)
      (else
        (`self.SpawnBall`)))))

(fn `SpawnBall`
  (bind _returnvalue (`|SpawnActorFromClass` "/Game/Actors/BP_Ball.BP_Ball_C" (`SceneComponent.K2_GetComponentToWorld` (`self.Capsule`)) "AlwaysSpawn" "OverrideRootScale" null null))
  (bind _output_get (set `self.PlayingBall` _returnvalue))
  (add `/Game/Actors/BP_Ball.OnDead` _output_get (`|CreateDelegate` :!event `OnBallDead`)))

(fn `SubstructLife`
  (locals (NewLocalVar_0 :type "Actor Object Reference"))
  (bind _output_get (set `self.Life` (- (`self.Life`) 1)))
  (`KismetSystemLibrary.PrintString` (`KismetStringLibrary.Concat_StrStr` "Number of lives: " (`KismetStringLibrary.Conv_IntToString` _output_get)) true true (struct :`R` 0.132949 :`G` 1.0 :`A` 1.0) 3.0))

(fn `UserConstructionScript`)