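; BP_Bonus is a moving pickup actor that makes the pawn spawn a ball when the two overlap.
; Each tick it moves with a swept world offset, using only the Y component of Direction times Speed scaled by delta time.
; On overlap, a BP_Pawn triggers SpawnBall and destroys the bonus, while a KillZVolume destroys it without any reward.
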(event `self.ReceiveActorBeginOverlap`
  (params (OtherActor :type "Actor Object Reference"))
  (`|ExecutionSequence`
    (:`then_0`
      (bind _asbp_pawn (cast `/Game/Actors/BP_Pawn` OtherActor))
      (`/Game/Actors/BP_Pawn.SpawnBall` _asbp_pawn))
    (:`then_1`
      (cast `KillZVolume` OtherActor)))
  (`self.K2_DestroyActor`))

(event `self.ReceiveTick`
  (params (DeltaSeconds :type "Float (single-precision)"))
  (bind (_returnvalue_x _returnvalue_y) (`KismetMathLibrary.BreakVector` (* (* (`self.Direction`) (`self.Speed`)) DeltaSeconds)))
  (`self.K2_AddActorWorldOffset` (`KismetMathLibrary.MakeVector` 0.0 _returnvalue_y) true))

(fn `UserConstructionScript`)